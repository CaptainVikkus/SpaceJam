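; First-person player pawn that walks, looks around, carries physics objects and presses buttons.
; Interact runs a short line trace from the eyes to grab or drop simulating objects, or calls Press on a Button otherwise.
; A PhysicsHandle pulls the held component to the Pivot's location every Tick.
; While Manipulate is held, look input rotates the held Pickup or BrokenPickUp cylinder instead of turning the view.
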(event Custom|PickupObject
  (params (Component :type Primitive%20Component%20Object%20Reference) (Pickup%20Actor :type Actor%20Object%20Reference))
  (Physics|Components|PhysicsHandle|GrabComponentatLocationwithRotation (Variables|Default|GetPhysicsHandle) Component "None" (Transformation|GetWorldLocation Component) (Math|Rotator|MakeRotator 0.0 0.0 0.0))
  (Variables|Default|SetIsHolding true)
  (Variables|Default|SetPickupActor Pickup%20Actor))

(event Custom|DropObject
  (Physics|Components|PhysicsHandle|ReleaseComponent (Variables|Default|GetPhysicsHandle))
  (Variables|Default|SetIsHolding false)
  (Variables|Default|SetPickupActor 0))

(event EventBeginPlay
  (Input|EnableInput (Game|GetPlayerController 0)))

(event Collision|EventActorBeginOverlap
  (params (OtherActor :type Actor%20Object%20Reference)))

(event EventTick
  (params (DeltaSeconds :type Float%20%28single-precision%29))
  (Physics|Components|PhysicsHandle|SetTargetLocation (Variables|Default|GetPhysicsHandle) (Transformation|GetWorldLocation (Variables|Default|GetPivot))))

(event Input|ActionEvents|InputActionInteract
  (params (Key :type Key%20Structure))
  (bind (_outlocation _outrotation) (Actor|GetActorEyesViewPoint))
  ;[1 1 1] Interact
  (:Pressed
    (bind (_outhit _returnvalue) (Collision|LineTraceByChannel _outlocation (+ _outlocation (* (Math|Vector|GetForwardVector _outrotation) 2e+02)) "TraceTypeQuery1" false 0 "None"))
    (if _returnvalue
      (if (Physics|IsSimulatingPhysics (.HitComponent (Collision|BreakHitResult _outhit)) "None")
        (if (Variables|Default|GetIsHolding)
          (CallFunction|DropObject)
          (else
            (CallFunction|PickupObject (.HitComponent (Collision|BreakHitResult _outhit)) (.HitActor (Collision|BreakHitResult _outhit)))))
        (else
          (bind _asbutton (Utilities|Casting|CastToButton (.HitActor (Collision|BreakHitResult _outhit))))
          (Default|Press _asbutton))))))

(event Input|ActionEvents|InputActionManipulate
  (params (Key :type Key%20Structure))
  (:Pressed
    (Variables|Default|SetClicking true))
  (:Released
    (Variables|Default|SetClicking false)))

(event Input|AxisEvents|InputAxisMoveRight
  (params (AxisValue :type Float%20%28single-precision%29))
  ;[1 1 1] Movement
  (Pawn|Input|AddMovementInput (Math|Vector|GetRightVector (Math|Rotator|MakeRotator 0.0 0.0 (.Yaw (Math|Rotator|BreakRotator (Pawn|GetControlRotation :!class /Script/Engine.Pawn))))) AxisValue false))

(event Input|AxisEvents|InputAxisMoveForward
  (params (AxisValue :type Float%20%28single-precision%29))
  ;[1 1 1] Movement
  (Pawn|Input|AddMovementInput (Math|Vector|GetForwardVector (Math|Rotator|MakeRotator 0.0 0.0 (.Yaw (Math|Rotator|BreakRotator (Pawn|GetControlRotation :!class /Script/Engine.Pawn))))) AxisValue false))

(event Input|AxisEvents|InputAxisTurn
  (params (AxisValue :type Float%20%28single-precision%29))
  (bind _returnvalue (* AxisValue -1e+01))
  (bind _pickupactor (Variables|Default|GetPickupActor))
  ;[1 1 1] Movement
  (if (Variables|Default|GetClicking)
    (Utilities|FlowControl|Sequence
      (:then_0
        (bind _aspickup (Utilities|Casting|CastToPickup _pickupactor))
        (Transformation|AddWorldRotation (Variables|/Game/LifeSupport/Actors/Pickup.Pickup_C|GetCylinder _aspickup) (Math|Rotator|MakeRotator (* (stale Input|AxisEvents|InputAxisLookUp AxisValue) -1e+01) 0.0 _returnvalue) false false))
      (:then_1
        (bind _asbroken_pick_up (Utilities|Casting|CastToBrokenPickUp _pickupactor))
        (Transformation|AddWorldRotation (Variables|/Game/LifeSupport/Actors/BrokenPickUp.BrokenPickUp_C|GetCylinder _asbroken_pick_up) (Math|Rotator|MakeRotator (* (stale Input|AxisEvents|InputAxisLookUp AxisValue) -1e+01) 0.0 _returnvalue) false false)))
    (else
      (Pawn|Input|AddControllerYawInput AxisValue))))

(event Input|AxisEvents|InputAxisLookUp
  (params (AxisValue :type Float%20%28single-precision%29))
  (bind _returnvalue (* AxisValue -1e+01))
  (bind _pickupactor (Variables|Default|GetPickupActor))
  ;[1 1 1] Movement
  (if (Variables|Default|GetClicking)
    (Utilities|FlowControl|Sequence
      (:then_0
        (bind _aspickup (Utilities|Casting|CastToPickup _pickupactor))
        (Transformation|AddWorldRotation (Variables|/Game/LifeSupport/Actors/Pickup.Pickup_C|GetCylinder _aspickup) (Math|Rotator|MakeRotator _returnvalue 0.0 (* (stale Input|AxisEvents|InputAxisTurn AxisValue) -1e+01)) false false))
      (:then_1
        (bind _asbroken_pick_up (Utilities|Casting|CastToBrokenPickUp _pickupactor))
        (Transformation|AddWorldRotation (Variables|/Game/LifeSupport/Actors/BrokenPickUp.BrokenPickUp_C|GetCylinder _asbroken_pick_up) (Math|Rotator|MakeRotator _returnvalue 0.0 (* (stale Input|AxisEvents|InputAxisTurn AxisValue) -1e+01)) false false)))
    (else
      (Pawn|Input|AddControllerPitchInput AxisValue))))

(fn ConstructionScript)