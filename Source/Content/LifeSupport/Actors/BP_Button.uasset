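; BP_Button is an interactable Life Support button that sets a smoke flag based on the pipe puzzle state.
; Player overlap with its capsule enables input and shows prompt text; leaving hides the text but calls EnableInput again, so input stays active.
; Pressing or releasing F updates Pressed and sets LetThereBeSmoke true only when CorrectPipes equals four.
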(event OnComponentBeginOverlap(Capsule)
  (params (OverlappedComponent :type Primitive%20Component%20Object%20Reference) (OtherActor :type Actor%20Object%20Reference) (OtherComp :type Primitive%20Component%20Object%20Reference) (OtherBodyIndex :type Integer) (bFromSweep :type Boolean) (SweepResult :type Hit%20Result%20Structure%20%28by%20ref%29))
  (Utilities|Casting|CastToBP_Player OtherActor)
  (Input|EnableInput (Game|GetPlayerController 0))
  (Rendering|SetVisibility (Variables|Default|GetTextRender) true false))

(event OnComponentEndOverlap(Capsule)
  (params (OverlappedComponent :type Primitive%20Component%20Object%20Reference) (OtherActor :type Actor%20Object%20Reference) (OtherComp :type Primitive%20Component%20Object%20Reference) (OtherBodyIndex :type Integer))
  (Utilities|Casting|CastToBP_Player OtherActor)
  (Input|EnableInput (Game|GetPlayerController 0))
  (Rendering|SetVisibility (Variables|Default|GetTextRender) false false))

(event EventBeginPlay)

(event Input|KeyboardEvents|F
  (params (Key :type Key%20Structure))
  (:Pressed
    (Variables|Default|SetPressed true)
    (if (== (Variables|Default|GetCorrectPipes) 4) :!label _label
      (Variables|Default|SetLetThereBeSmoke true)
      (else
        (Variables|Default|SetLetThereBeSmoke false))))
  (:Released
    (Variables|Default|SetPressed false)
    (goto _label)))

(fn ConstructionScript)