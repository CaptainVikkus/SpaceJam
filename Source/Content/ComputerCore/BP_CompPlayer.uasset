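; Player pawn for the computer core, with camera look, movement and interaction with data banks.
; Each tick, a sphere trace from the camera highlights the targeted interactable by toggling custom depth on its "Outline"-tagged component, with a DoOnce clearing it when the trace misses.
; Interact traces to toggle a BP_DataBank's interacting state or trigger a DB_Manager check.
; Manipulate purges a data bank that is being interacted with and not yet purged.
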(event EventBeginPlay
  ;[1 1 1] Begin Play
  (Input|EnableInput (Game|GetPlayerController 0)))

(event EventTick
  (params (DeltaSeconds :type Float%20%28single-precision%29))
  (bind _camera (Variables|Default|GetCamera))
  (bind _returnvalue (Transformation|GetWorldLocation _camera))
  ;[1 1 1] Tracing
  (bind (_outhit _returnvalue_2) (Collision|SphereTraceForObjects _returnvalue (+ _returnvalue (* (Math|Vector|GetForwardVector (Pawn|GetControlRotation :!class /Script/Engine.Pawn)) 5e+02)) 1e+01 (Utilities|Array|MakeArray "ObjectTypeQuery8") false 0 "None"))
  (if _returnvalue_2
    (if (== (.hitactor (Variables|Default|GetHitInteractable)) (.HitActor (Collision|BreakHitResult _outhit)))
      _
      (else
        (CallFunction|StartTracing (.HitActor (Collision|BreakHitResult _outhit)) (.hitactor (Variables|Default|GetHitInteractable)))))
    (Variables|Default|SetHitInteractable _outhit)
    (goto _label Reset)
    (else
      (Utilities|FlowControl|DoOnce false :!label _label
        (:Completed
          (CallFunction|EndTracing))))))

(event Input|ActionEvents|InputActionManipulate
  (params (Key :type Key%20Structure))
  (bind _camera (Variables|Default|GetCamera))
  (bind _returnvalue (Transformation|GetWorldLocation _camera))
  ;[1 1 1] DataBank Interaction
  (:Pressed
    (bind (_outhit _returnvalue_2) (Collision|SphereTraceForObjects _returnvalue (+ _returnvalue (* (Math|Vector|GetForwardVector (Pawn|GetControlRotation :!class /Script/Engine.Pawn)) 1e+03)) 0.0 (Utilities|Array|MakeArray "ObjectTypeQuery1") false 0 "None"))
    (if _returnvalue_2
      (bind _asbp_data_bank (Utilities|Casting|CastToBP_DataBank (.HitActor (Collision|BreakHitResult _outhit))))
      (if (Variables|/Game/ComputerCore/BP_DataBank.BP_DataBank_C|GetInteracting _asbp_data_bank)
        (if (not (Variables|/Game/ComputerCore/BP_DataBank.BP_DataBank_C|GetPurged _asbp_data_bank))
          (Default|Purge _asbp_data_bank))))))

(event Input|ActionEvents|InputActionInteract
  (params (Key :type Key%20Structure))
  (bind _camera (Variables|Default|GetCamera))
  (bind _returnvalue (Transformation|GetWorldLocation _camera))
  ;[1 1 1] DataBank Interaction
  (:Pressed
    (bind (_outhit _returnvalue_2) (Collision|SphereTraceForObjects _returnvalue (+ _returnvalue (* (Math|Vector|GetForwardVector (Pawn|GetControlRotation :!class /Script/Engine.Pawn)) 1e+03)) 1e+01 (Utilities|Array|MakeArray "ObjectTypeQuery1") false 0 "None"))
    (if _returnvalue_2
      (bind _asbp_data_bank (Utilities|Casting|CastToBP_DataBank (.HitActor (Collision|BreakHitResult _outhit)))
        (:then
          (if (Variables|/Game/ComputerCore/BP_DataBank.BP_DataBank_C|GetInteracting _asbp_data_bank)
            (Variables|/Game/ComputerCore/BP_DataBank.BP_DataBank_C|SetInteracting _asbp_data_bank false)
            (else
              (Variables|/Game/ComputerCore/BP_DataBank.BP_DataBank_C|SetInteracting _asbp_data_bank true)))
          (Default|Interacted _asbp_data_bank))
        (:CastFailed
          (bind _asdb_manager (Utilities|Casting|CastToDB_Manager (.HitActor (Collision|BreakHitResult _outhit)))
            (:then
              (Default|Checking _asdb_manager))
            (:CastFailed
              (Development|PrintString "Hello"))))))))

(event Input|AxisEvents|InputAxisTurn
  (params (AxisValue :type Float%20%28single-precision%29))
  ;[1 1 1] Camera Functionality
  (Pawn|Input|AddControllerYawInput AxisValue))

(event Input|AxisEvents|InputAxisLookUp
  (params (AxisValue :type Float%20%28single-precision%29))
  ;[1 1 1] Camera Functionality
  (Pawn|Input|AddControllerPitchInput AxisValue))

(event Input|AxisEvents|InputAxisMoveForward
  (params (AxisValue :type Float%20%28single-precision%29))
  ;[1 1 1] Movement Inputs
  (Pawn|Input|AddMovementInput (Math|Vector|GetForwardVector (Math|Rotator|MakeRotator 0.0 0.0 (.Yaw (Math|Rotator|BreakRotator (Pawn|GetControlRotation :!class /Script/Engine.Pawn))))) AxisValue false))

(event Input|AxisEvents|InputAxisMoveRight
  (params (AxisValue :type Float%20%28single-precision%29))
  ;[1 1 1] Movement Inputs
  (Pawn|Input|AddMovementInput (Math|Vector|GetRightVector (Math|Rotator|MakeRotator 0.0 0.0 (.Yaw (Math|Rotator|BreakRotator (Pawn|GetControlRotation :!class /Script/Engine.Pawn))))) AxisValue false))

(fn ConstructionScript)

(fn StartTracing
  (params (NewActor :type Actor%20Object%20Reference) (OldActor :type Actor%20Object%20Reference))
  (Rendering|SetRenderCustomDepth (Utilities|Array|Get(acopy) (Actor|GetComponentsbyTag NewActor "/Script/Engine.PrimitiveComponent" "Outline")) true)
  (if (not (== OldActor 0))
    (Rendering|SetRenderCustomDepth (Utilities|Array|Get(acopy) (Actor|GetComponentsbyTag OldActor "/Script/Engine.PrimitiveComponent" "Outline")) false)))

(fn EndTracing
  (Utilities|FlowControl|Sequence
    (:then_0
      (if (not (== (.hitactor (Variables|Default|GetHitInteractable)) 0))
        (Rendering|SetRenderCustomDepth (Actor|GetComponentsbyTag (.hitactor (Variables|Default|GetHitInteractable)) "/Script/Engine.PrimitiveComponent" "Outline") false)))
    (:then_1
      (Variables|Default|SetHitInteractable ""))))